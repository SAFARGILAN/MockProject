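; VR player sample for an on-rails shooter, carried along BP_Spline by the Move timeline, which sets capsule location and rotation.
; The right trigger action spends Ammo to spawn projectiles from the Gun with sound and haptics; a fast right-controller motion along Y refills it.
; Enemies entering the left or right box spawn directional arrow indicators, while touching the player only plays a sound, as damage handling is unwired.
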(event OnComponentBeginOverlap(BoxLeft)
  (params (OverlappedComponent :type Primitive%20Component%20Object%20Reference) (OtherActor :type Actor%20Object%20Reference) (OtherComp :type Primitive%20Component%20Object%20Reference) (OtherBodyIndex :type Integer) (bFromSweep :type Boolean) (SweepResult :type Hit%20Result%20Structure%20%28by%20ref%29))
  (if (Actor|ActorHasTag OtherActor "Enemy")
    (Utilities|FlowControl|DoOnce false :!label _label
      (:Completed
        (Game|SpawnActorfromClass "/Game/SafaFolder/BP_LeftArrow.BP_LeftArrow_C" (Transformation|GetWorldTransform (Variables|Default|GetCube)) "Undefined" "MultiplyWithRoot" 0 0)
        (goto _label Reset)))))

(event OnComponentBeginOverlap(BoxRight)
  (params (OverlappedComponent :type Primitive%20Component%20Object%20Reference) (OtherActor :type Actor%20Object%20Reference) (OtherComp :type Primitive%20Component%20Object%20Reference) (OtherBodyIndex :type Integer) (bFromSweep :type Boolean) (SweepResult :type Hit%20Result%20Structure%20%28by%20ref%29))
  (if (Actor|ActorHasTag OtherActor "Enemy")
    (Utilities|FlowControl|DoOnce false :!label _label
      (:Completed
        (Game|SpawnActorfromClass "/Game/SafaFolder/BP_RightArrow.BP_RightArrow_C" (Transformation|GetWorldTransform (Variables|Default|GetCube)) "Undefined" "MultiplyWithRoot" 0 0)
        (goto _label Reset)))))

(event Input|EnhancedActionEvents|EnhancedInputActionIA_Hand_Grasp_Right
  (params (ActionValue :type Float%20%28double-precision%29) (ElapsedSeconds :type Float%20%28double-precision%29) (TriggeredSeconds :type Float%20%28double-precision%29) (InputAction :type Input%20Action%20Object%20Reference :default "/Game/VRTemplate/Input/Actions/Hands/IA_Hand_Grasp_Right.IA_Hand_Grasp_Right")))

(event Input|EnhancedActionEvents|EnhancedInputActionIA_Shoot_Right
  (params (ActionValue :type Boolean) (ElapsedSeconds :type Float%20%28double-precision%29) (TriggeredSeconds :type Float%20%28double-precision%29) (InputAction :type Input%20Action%20Object%20Reference :default "/Game/VRTemplate/Input/Actions/IA_Shoot_Right.IA_Shoot_Right"))
  (:Started
    (if (not (<= (Variables|Default|GetAmmo) 0))
      (Variables|Default|SetAmmo (- (Variables|Default|GetAmmo) 1))
      ;[0.03434 0.03434 0.03434] Spawn the projectile
      (Game|SpawnActorfromClass "/Game/SafaFolder/Projectile.Projectile_C" (Math|Transform|MakeTransform (Transformation|GetWorldLocation (Variables|Default|GetGun)) (Transformation|GetWorldRotation (Variables|Default|GetRightController))) "Undefined" "OverrideRootScale" self (Game|Player|GetPlayerPawn 0))
      (Audio|PlaySoundatLocation "/Game/SafaFolder/ショット.ショット" (Transformation|GetWorldLocation (Variables|Default|GetRightController)) "0, 0, 0" 1.0 1.0 0.0 0 0 0 0)
      (Class|PlayerController|PlayHapticEffect (Game|GetPlayerController 0) (Variables|Default|GetPistolFireHapticEffect) "Right" 5e+01 false))))

(event EventBeginPlay
  (if (Class|HeadMountedDisplayFunctionLibrary|IsHeadMountedDisplayEnabled)
    (Class|HeadMountedDisplayFunctionLibrary|SetTrackingOrigin "View")))

(event Collision|EventActorBeginOverlap
  (params (OtherActor :type Actor%20Object%20Reference))
  (if (Actor|ActorHasTag OtherActor "Enemy")
    (Audio|PlaySound2D "/Game/SafaFolder/「ぐっ！」.「ぐっ！」" 1.0 1.0 0.0 0 0)))

(event EventTick
  (params (DeltaSeconds :type Float%20%28single-precision%29))
  (bind _capsulecomponent (Variables|Default|GetCapsuleComponent))
  (bind _returnvalue (Actor|GetActorOfClass "/Game/SafaFolder/BP_Spline.BP_Spline_C"))
  (bind _newtrack_2 (Timeline|Move Play)
    (:Update
      (Variables|Default|SetDistance (* _newtrack_2 (Spline|GetSplineLength (Variables|/Game/SafaFolder/BP_Spline.BP_Spline_C|GetSpline _returnvalue))))
      (Transformation|SetWorldLocation _capsulecomponent (Spline|GetLocationatDistanceAlongSpline (Variables|/Game/SafaFolder/BP_Spline.BP_Spline_C|GetSpline _returnvalue) (Variables|Default|GetDistance) "World") false false)
      (Transformation|SetWorldRotation _capsulecomponent (Spline|GetRotationatDistanceAlongSpline (Variables|/Game/SafaFolder/BP_Spline.BP_Spline_C|GetSpline _returnvalue) (Variables|Default|GetDistance) "World") false false)
      (if (>= (.y (.OutLinearVelocity (Class|MotionControllerComponent|GetLinearVelocity (Variables|Default|GetRightController)))) 9e+01)
        (Class|PlayerController|PlayHapticEffect (Game|GetPlayerController 0) (Variables|Default|GetPistolFireHapticEffect) "Right" 5e+02 false)
        (Audio|PlaySound2D "/Game/SafaFolder/パワーアップ.パワーアップ" 1.0 1.0 0.0 0 0)
        (Variables|Default|SetAmmo (Variables|Default|GetAmmoMax))))))

(event EventGetHit)

(fn ConstructionScript)