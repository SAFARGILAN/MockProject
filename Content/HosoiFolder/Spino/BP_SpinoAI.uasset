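; AI controller for the BP_Spino enemy, driving it with the BT_Spino behavior tree.
; On possess it starts the tree, caches the Spino as its owner and writes that pawn's player target to the Blackboard.
; Every tick it mirrors the Spino's timer and near-player flag into the Blackboard as the wait time and attacking state.
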(event EventTick
  (params (DeltaSeconds :type Float%20%28single-precision%29))
  ;[1 1 1] BlackBoardのWaitTimeの更新
  (AI|Components|Blackboard|SetValueasFloat (Variables|Default|GetBlackboard) (Utilities|Name|MakeLiteralName "WaitTime") (Variables|/Game/HosoiFolder/Spino/BP_Spino.BP_Spino_C|GetEnemyTimer (Variables|Default|GetMyOwner)))
  ;[1 1 1] IsAttackingの更新
  (AI|Components|Blackboard|SetValueasBool (Variables|Default|GetBlackboard) (Utilities|Name|MakeLiteralName "IsAttacking") (Variables|/Game/HosoiFolder/Spino/BP_Spino.BP_Spino_C|GetIsNearPlayer (Variables|Default|GetMyOwner))))

(event EventPossess
  (params (PossessedPawn :type Pawn%20Object%20Reference))
  (AI|RunBehaviorTree "/Game/HosoiFolder/Spino/AI/BT_Spino.BT_Spino")
  ;[1 1 1] MyOwnerの設定
  (bind _asbp_spino (Utilities|Casting|CastToBP_Spino (Components|GetOwner (Variables|/Script/Engine.Actor|GetRootComponent PossessedPawn)))
    (:then
      (Variables|Default|SetMyOwner _asbp_spino)
      ;[1 1 1] BlackBoardにPlayerをセットする
      (AI|Components|Blackboard|SetValueasObject (Variables|Default|GetBlackboard) (Utilities|Name|MakeLiteralName "Target") (Variables|/Game/HosoiFolder/Spino/BP_Spino.BP_Spino_C|GetTarget (Variables|Default|GetMyOwner))))
    (:CastFailed
      (Development|PrintString "Cast失敗"))))

(fn ConstructionScript)