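; BP_SampleEnemy is a sample enemy character that targets BP_Player2 and dies in one hit.
; Tick counts down about once per second via a Delay to set IsRun, and sets IsNearPlayer when the target is within SearchRange.
; AttackCollider sends GetHitMessage once, gated by IsFirstAttack; GetHit stops movement and destroys the actor after a delay.
; MoveStraight uses SimpleMoveToActor toward the target but is not called within this Blueprint.
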(event OnComponentBeginOverlap(AttackCollider)
  (params (OverlappedComponent :type Primitive%20Component%20Object%20Reference) (OtherActor :type Actor%20Object%20Reference) (OtherComp :type Primitive%20Component%20Object%20Reference) (OtherBodyIndex :type Integer) (bFromSweep :type Boolean) (SweepResult :type Hit%20Result%20Structure%20%28by%20ref%29))
  ;[1 1 1] プレイヤーとぶつかったときの処理(Colliderが自身のカプセルに被ってると自分のGetHitが呼ばれるので注意)
  (if (Variables|Default|GetIsFirstAttack)
    (Class|BPIGetHit|GetHit(Message) OtherActor)
    (Variables|Default|SetIsFirstAttack false)))

(event EventGetHit
  ;[1 1 1] 攻撃を食らった時の処理
  (Variables|Default|SetIsDead true)
  (Development|PrintString "敵死亡")
  (bind _output_get (Variables|Default|SetMoveSpeed 0.0))
  (Variables|/Script/Engine.CharacterMovementComponent|SetMaxWalkSpeed (Variables|Character|GetCharacterMovement) _output_get)
  (Utilities|FlowControl|Delay 5.0)
  (Actor|DestroyActor))

(event EventBeginPlay
  ;[1 1 1] ターゲットを設定
  (bind _returnvalue (Actor|GetActorOfClass "/Game/SafaFolder/BP_Player2.BP_Player2_C"))
  (Variables|Default|SetTarget _returnvalue)
  ;[1 1 1] 移動スピードを設定
  (Variables|/Script/Engine.CharacterMovementComponent|SetMaxWalkSpeed (Variables|Character|GetCharacterMovement) (Variables|Default|GetMoveSpeed)))

(event EventTick
  (params (DeltaSeconds :type Float%20%28single-precision%29))
  (bind _enemytimer (Variables|Default|GetEnemyTimer))
  (Utilities|FlowControl|Sequence
    (:then_0
      ;[1 1 1] 一定時間待つ
      (Utilities|FlowControl|Delay 1.0)
      (Math|Float|DecrementFloat _enemytimer
        (:%20%20
          (if (<= _enemytimer 0.0)
            ;[1 1 1] IsRunをtrueに変更する
            (if (not (Variables|Default|GetIsRun))
              (Variables|Default|SetIsRun true)
              (Development|PrintString "走ります！"))))))
    (:then_1
      (if (<= (Math|Vector|VectorLength (- (.location (Transformation|GetActorTransform (Variables|Default|GetTarget))) (.location (Transformation|GetActorTransform)))) (Variables|Default|GetSearchRange))
        ;[1 1 1] 攻撃を開始させる
        (if (not (Variables|Default|GetIsNearPlayer))
          (Variables|Default|SetIsNearPlayer true))))))

(fn ConstructionScript)

(fn MoveStraight
  ;[1 1 1] 直進させる
  (AI|Navigation|SimpleMovetoActor (Pawn|GetController) (Variables|Default|GetTarget)))