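; BP_SampleEnemyAI is the AI controller for the sample enemy.
; On possess it runs BT_Enemy and caches the pawn as BP_SampleEnemy, printing an error if the cast fails.
; Every tick it copies the enemy's EnemyTimer and IsNearPlayer into the WaitTime and IsAttacking Blackboard keys, so the pawn's state feeds the behavior tree.
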(event EventTick
  (params (DeltaSeconds :type Float%20%28single-precision%29))
  ;[1 1 1] BlackBoardのWaitTimeの更新
  (AI|Components|Blackboard|SetValueasFloat (Variables|Default|GetBlackboard) (Utilities|Name|MakeLiteralName "WaitTime") (Variables|/Game/HosoiFolder/BluePrint/Enemy/BP_SampleEnemy.BP_SampleEnemy_C|GetEnemyTimer (Variables|Default|GetMyOwner)))
  ;[1 1 1] IsAttackingの更新
  (AI|Components|Blackboard|SetValueasBool (Variables|Default|GetBlackboard) (Utilities|Name|MakeLiteralName "IsAttacking") (Variables|/Game/HosoiFolder/BluePrint/Enemy/BP_SampleEnemy.BP_SampleEnemy_C|GetIsNearPlayer (Variables|Default|GetMyOwner))))

(event EventPossess
  (params (PossessedPawn :type Pawn%20Object%20Reference))
  (AI|RunBehaviorTree "/Game/HosoiFolder/BluePrint/Enemy/AI/BT_Enemy.BT_Enemy")
  ;[1 1 1] MyOwnerの設定
  (bind _asbp_sample_enemy (Utilities|Casting|CastToBP_SampleEnemy (Components|GetOwner (Variables|/Script/Engine.Actor|GetRootComponent PossessedPawn)))
    (:then
      (Variables|Default|SetMyOwner _asbp_sample_enemy))
    (:CastFailed
      (Development|PrintString "Cast失敗"))))

(fn ConstructionScript)