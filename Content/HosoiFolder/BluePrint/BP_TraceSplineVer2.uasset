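; BP_TraceSplineVer2 is a spline path Blueprint that serves world-space location and rotation queries, apparently for tracing along the spline.
; GetCurrentLocation wraps the input distance by spline length when looping, otherwise uses zero, and returns the location and resulting distance.
; GetCurrentRotation takes no input and samples spline rotation at LocalDistance.
; The event graph and construction script contain no logic, so any movement happens outside this Blueprint.
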(event EventBeginPlay)

(event Collision|EventActorBeginOverlap
  (params (OtherActor :type Actor%20Object%20Reference)))

(event EventTick
  (params (DeltaSeconds :type Float%20%28single-precision%29)))

(fn ConstructionScript)

(fn GetCurrentLocation
  (params (InputLength :type Float%20%28double-precision%29) (IsLoop :type Boolean))
  (if IsLoop
    (Variables|Default|SetLocalDistance (Math|Float|%(Float) InputLength (Spline|GetSplineLength (Variables|Default|GetSpline))))
    (else
      (Variables|Default|SetLocalDistance 0.0)))
  (return (Spline|GetLocationatDistanceAlongSpline (Variables|Default|GetSpline) (Variables|Default|GetLocalDistance) "World") (Variables|Default|GetLocalDistance)))

(fn GetCurrentRotation
  (return (Spline|GetRotationatDistanceAlongSpline (Variables|Default|GetSpline) (Variables|Default|GetLocalDistance) "World")))