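; Older enemy AI controller that starts the BT_SampleEnemy_Old behavior tree on BeginPlay.
; Its perception update loops over updated actors and compares each to BP_Player, but does nothing with a match.
; Disconnected nodes hold sight found/lost logic that would set the blackboard State enum, assign VRPawn as Target or clear it, and print debug messages.
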(event OnPerceptionUpdated(AIPerception)
  (params (UpdatedActors :type Array%20of%20Actor%20Object%20References))
  ;[1 1 1] 視界情報のアップデート判定
  (for _array_element UpdatedActors
    (bind _returnvalue (Actor|GetActorOfClass "/Game/SafaFolder/BP_Player.BP_Player_C"))
    (if (== _returnvalue _array_element)
      _)))

(event EventBeginPlay
  (AI|RunBehaviorTree "/Game/HosoiFolder/BluePrint/Enemy_A/AI/BT_SampleEnemy_Old.BT_SampleEnemy_Old"))

(fn ConstructionScript)