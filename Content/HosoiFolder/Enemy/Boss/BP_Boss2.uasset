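; BP_Boss2 is a boss enemy character that roars after spawning and then becomes able to walk.
; BeginPlay caches BP_Player2 as Target, waits WaitTime to set CanRage, then after a fixed delay enables CanWalk and applies MoveSpeed.
; While CanWalk is true, Tick accumulates RageTimer and periodically plays a rage sound at the boss.
; Several chase and look-at rotation experiments remain disconnected, so this graph does not move the boss.
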(event EventBeginPlay
  ;[1 1 1] 吠える
  (bind _returnvalue (Actor|GetActorOfClass "/Game/SafaFolder/BP_Player2.BP_Player2_C"))
  (Variables|Default|SetTarget _returnvalue)
  (Utilities|FlowControl|Delay (Variables|Default|GetWaitTime))
  (Variables|Default|SetCanRage true)
  (Utilities|FlowControl|Delay 3.2)
  (Variables|Default|SetCanWalk true)
  ;[1 1 1] 移動スピードを設定
  (Variables|/Script/Engine.CharacterMovementComponent|SetMaxWalkSpeed (Variables|Character|GetCharacterMovement) (Variables|Default|GetMoveSpeed)))

(event EventTick
  (params (DeltaSeconds :type Float%20%28single-precision%29))
  ;[1 1 1] プレイヤーの方向に移動
  (if (Variables|Default|GetCanWalk)
    ;[1 1 1] 一定時間を超えたら叫ばせる
    (Variables|Default|SetRageTimer (+ DeltaSeconds (Variables|Default|GetRageTimer)))
    (if (>= (Variables|Default|GetRageTimer) 1e+01)
      (Variables|Default|SetRageTimer 0.0)
      (Audio|PlaySoundatLocation "/Game/HosoiFolder/Enemy/Boss/SE_BossRage.SE_BossRage" (Transformation|GetActorLocation) "0, 0, 0" 1.0 1.0 0.0 0 0 0 0))))

(fn ConstructionScript)