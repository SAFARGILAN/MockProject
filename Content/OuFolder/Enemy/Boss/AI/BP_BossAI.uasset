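; BP_BossAI is the AI controller for the boss enemy, running the BT_Boss behavior tree when it possesses a pawn.
; On possess it caches the BP_Boss2 owner and writes that boss's Target to the Blackboard, printing a failure message if the cast fails.
; Every tick it mirrors the boss's CanWalk flag into the Blackboard for the tree to read.
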(event EventTick
  (params (DeltaSeconds :type Float%20%28single-precision%29))
  ;[1 1 1] BlackBoardのCanWalkの更新
  (AI|Components|Blackboard|SetValueasBool (Variables|Default|GetBlackboard) (Utilities|Name|MakeLiteralName "CanWalk") (Variables|/Game/HosoiFolder/Enemy/Boss/BP_Boss2.BP_Boss2_C|GetCanWalk (Variables|Default|GetMyOwner))))

(event EventPossess
  (params (PossessedPawn :type Pawn%20Object%20Reference))
  (AI|RunBehaviorTree "/Game/HosoiFolder/Enemy/Boss/AI/BT_Boss.BT_Boss")
  ;[1 1 1] MyOwnerの設定
  (bind _asbp_boss_2 (Utilities|Casting|CastToBP_Boss2 (Components|GetOwner (Variables|/Script/Engine.Actor|GetRootComponent PossessedPawn)))
    (:then
      (Variables|Default|SetMyOwner _asbp_boss_2)
      ;[1 1 1] BlackBoardにPlayerをセットする
      (AI|Components|Blackboard|SetValueasObject (Variables|Default|GetBlackboard) (Utilities|Name|MakeLiteralName "Target") (Variables|/Game/HosoiFolder/Enemy/Boss/BP_Boss2.BP_Boss2_C|GetTarget (Variables|Default|GetMyOwner))))
    (:CastFailed
      (Development|PrintString "Cast失敗"))))

(fn ConstructionScript)