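; BP_Boss1 is a scripted boss enemy that roars, moves away and then disappears.
; BeginPlay runs a timed chain: after a wait it prints a roar message and sets CanRage, shortly after sets CanWalk, and later destroys the actor.
; While CanWalk is true, Tick slides it along world negative Y with a fixed, unswept per-frame offset, independent of delta time.
; A SimpleMoveToActor call is left unconnected.
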(event EventBeginPlay
  ;[1 1 1] 吠える→消える
  (Utilities|FlowControl|Delay 2e+01)
  (Development|PrintString "Bossが吠えました")
  (Variables|Default|SetCanRage true)
  (Utilities|FlowControl|Delay 3.6)
  (Variables|Default|SetCanWalk true)
  (Utilities|FlowControl|Delay 1e+01)
  (Actor|DestroyActor))

(event EventTick
  (params (DeltaSeconds :type Float%20%28single-precision%29))
  ;[1 1 1] 後ろに移動させる
  (if (Variables|Default|GetCanWalk)
    (Transformation|AddActorWorldOffset "0.000000,-100.000000,0.000000")))

(fn ConstructionScript)