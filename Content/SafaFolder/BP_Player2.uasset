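; BP_Player2 is a VR player pawn that rides a spline rail and shoots projectiles.
; Tick places the capsule on BP_Spline at a distance derived from game time and Speed, matching location and rotation.
; Right-hand shoot input spawns a projectile at the controller, with sound and haptics.
; Overlaps check Enemy, Player and Weapon tags through class lookups, then show a damage screen widget and print a hit message.
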(event Input|EnhancedActionEvents|EnhancedInputActionIA_Shoot_Right
  (params (ActionValue :type Boolean) (ElapsedSeconds :type Float%20%28double-precision%29) (TriggeredSeconds :type Float%20%28double-precision%29) (InputAction :type Input%20Action%20Object%20Reference :default "/Game/VRTemplate/Input/Actions/IA_Shoot_Right.IA_Shoot_Right"))
  (bind _rightcontroller (Variables|Default|GetRightController))
  (:Started
    ;[0.03434 0.03434 0.03434] Spawn the projectile
    (Game|SpawnActorfromClass "/Game/SafaFolder/Projectile.Projectile_C" (Math|Transform|MakeTransform (Transformation|GetWorldLocation _rightcontroller) (Transformation|GetWorldRotation _rightcontroller)) "Undefined" "OverrideRootScale" self (Game|Player|GetPlayerPawn 0))
    (Audio|PlaySoundatLocation "/Game/SafaFolder/ショット.ショット" (Transformation|GetWorldLocation (Variables|Default|GetRightController)) "0, 0, 0" 1.0 1.0 0.0 0 0 0 0)
    (Class|PlayerController|PlayHapticEffect (Game|GetPlayerController 0) (Variables|Default|GetPistolFireHapticEffect) "Right" 2e+01 false)))

(event EventBeginPlay
  (if (Class|HeadMountedDisplayFunctionLibrary|IsHeadMountedDisplayEnabled)
    (Class|HeadMountedDisplayFunctionLibrary|SetTrackingOrigin "View")))

(event Collision|EventActorBeginOverlap
  (params (OtherActor :type Actor%20Object%20Reference))
  (bind _returnvalue (Actor|GetActorOfClass "/Game/SafaFolder/BP_Weapon.BP_Weapon_C"))
  (bind _returnvalue_2 (Actor|GetActorOfClass (Utilities|GetClass OtherActor)))
  (if (Math|Boolean|ANDBoolean (Actor|ActorHasTag _returnvalue_2 "Enemy") (Actor|ActorHasTag "Player") (!= (Actor|ActorHasTag _returnvalue "Weapon") false))
    (bind _returnvalue_3 (UserInterface|CreateWidget "/Game/SafaFolder/WB_DammageScreen.WB_DammageScreen_C"))
    (UserInterface|Viewport|AddtoViewport _returnvalue_3 0)
    (Development|PrintString "攻撃を食らった")))

(event EventTick
  (params (DeltaSeconds :type Float%20%28single-precision%29))
  (bind _capsulecomponent (Variables|Default|GetCapsuleComponent))
  (bind _returnvalue (Actor|GetActorOfClass "/Game/SafaFolder/BP_Spline.BP_Spline_C"))
  (Variables|Default|SetDistance (* (+ (Utilities|Time|GetGameTimeinSeconds) (Utilities|Time|GetWorldDeltaSeconds)) (Variables|Default|GetSpeed)))
  (Transformation|SetWorldLocation _capsulecomponent (Spline|GetLocationatDistanceAlongSpline (Variables|/Game/SafaFolder/BP_Spline.BP_Spline_C|GetSpline _returnvalue) (Variables|Default|GetDistance) "World") false false)
  (Transformation|SetWorldRotation _capsulecomponent (Spline|GetRotationatDistanceAlongSpline (Variables|/Game/SafaFolder/BP_Spline.BP_Spline_C|GetSpline _returnvalue) (Variables|Default|GetDistance) "World") false false))

(event EventGetHit)

(fn ConstructionScript)