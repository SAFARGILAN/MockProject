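; VR tutorial player that, after five seconds of game time, walks forward automatically and can reload by moving the right controller quickly.
; Holding the right shoot input runs a looping timer that spends ammo to spawn projectiles with sound and haptics.
; A velocity threshold with DoOnce refills ammo once per swing.
; Enemy overlap shows a damage widget, gated until a non-enemy overlap resets it; the Move timeline is disconnected.
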(event Custom|OnFire
  (if (not (<= (Variables|Default|GetAmmo) 0))
    (Variables|Default|SetAmmo (- (Variables|Default|GetAmmo) 1))
    ;[0.03434 0.03434 0.03434] Spawn the projectile
    (Game|SpawnActorfromClass "/Game/SafaFolder/Projectile.Projectile_C" (Math|Transform|MakeTransform (Transformation|GetWorldLocation (Variables|Default|GetGun)) (Transformation|GetWorldRotation (Variables|Default|GetRightController))) "Undefined" "OverrideRootScale" self (Game|Player|GetPlayerPawn 0))
    (Audio|PlaySoundatLocation "/Game/SafaFolder/ショット.ショット" (Transformation|GetWorldLocation (Variables|Default|GetRightController)) "0, 0, 0" 1.0 1.0 0.0 0 0 0 0)
    (Class|PlayerController|PlayHapticEffect (Game|GetPlayerController 0) (Variables|Default|GetPistolFireHapticEffect) "Right" 5e+01 false)))

(event Input|EnhancedActionEvents|EnhancedInputActionIA_Shoot_Right
  (params (ActionValue :type Boolean) (ElapsedSeconds :type Float%20%28double-precision%29) (TriggeredSeconds :type Float%20%28double-precision%29) (InputAction :type Input%20Action%20Object%20Reference :default "/Game/VRTemplate/Input/Actions/IA_Shoot_Right.IA_Shoot_Right"))
  (:Started
    (bind _returnvalue (Utilities|Time|SetTimerbyEvent (delegate Custom|OnFire) 0.1 true))
    (Variables|Default|SetNewVar_2 _returnvalue)
    (CallFunction|OnFire))
  (:Canceled
    (Utilities|Time|ClearandInvalidateTimerbyHandle (Variables|Default|GetNewVar_2) :!label _label))
  (:Completed
    (goto _label)))

(event EventBeginPlay
  (if (Class|HeadMountedDisplayFunctionLibrary|IsHeadMountedDisplayEnabled)
    (Class|HeadMountedDisplayFunctionLibrary|SetTrackingOrigin "View")))

(event Collision|EventActorBeginOverlap
  (params (OtherActor :type Actor%20Object%20Reference))
  (if (Actor|ActorHasTag OtherActor "Enemy")
    (Variables|Default|SetIsHurt? true)
    (Utilities|FlowControl|DoOnce false :!label _label
      (:Completed
        (bind _returnvalue (UserInterface|CreateWidget "/Game/SafaFolder/WB_DammageScreen.WB_DammageScreen_C"))
        (UserInterface|Viewport|AddtoViewport _returnvalue 0)
        (Development|PrintString "攻撃を食らった")))
    (else
      (Variables|Default|SetIsHurt? false)
      (goto _label Reset))))

(event EventTick
  (params (DeltaSeconds :type Float%20%28single-precision%29))
  (if (>= (Utilities|Time|GetGameTimeinSeconds) 5.0)
    (Pawn|Input|AddMovementInput (Math|Vector|GetForwardVector (Variables|Default|GetCapsuleComponent)) 1.0 false)
    (if (>= (Math|Vector|VectorLength (.OutLinearVelocity (Class|MotionControllerComponent|GetLinearVelocity (Variables|Default|GetRightController)))) 9e+01)
      (Variables|Default|SetIsReloaded%20? true)
      (Utilities|FlowControl|DoOnce false :!label _label
        (:Completed
          (Class|PlayerController|PlayHapticEffect (Game|GetPlayerController 0) (Variables|Default|GetPistolFireHapticEffect) "Right" 5e+02 false)
          (Audio|PlaySound2D "/Game/SafaFolder/パワーアップ.パワーアップ" 1.0 1.0 0.0 0 0)
          (Variables|Default|SetAmmo (Variables|Default|GetAmmoMax))
          (Development|PrintString "Hello")
          (Variables|Default|SetIsReloaded%20? false)))
      (else
        (Variables|Default|SetIsReloaded%20? false)
        (goto _label Reset)))))

(event EventGetHit)

(fn ConstructionScript)