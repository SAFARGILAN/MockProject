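; BP_RedFlash is a component that briefly flashes its owning actor red when an actor tagged Player overlaps it.
; On BeginPlay it binds to the owner's begin-overlap event and creates a dynamic material instance on element 0 of the owner's skeletal mesh.
; The flash raises emissive color and multiplier parameters, then resets them to black and zero after a short delay.
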(event Custom|FlashRed
  (params (OverlappedActor :type Actor%20Object%20Reference) (OtherActor :type Actor%20Object%20Reference))
  (bind _flashmat (Variables|Default|GetFlashMat))
  (if (Actor|ActorHasTag OtherActor "Player")
    (Rendering|Material|SetVectorParameterValue _flashmat "EmissiveColor" "(R=1.000000,G=0.009362,B=0.000000,A=1.000000)" :!class /Script/Engine.MaterialInstanceDynamic)
    (Rendering|Material|SetScalarParameterValue _flashmat "EmissiveMultiplier" 15.0 :!class /Script/Engine.MaterialInstanceDynamic)
    (Utilities|FlowControl|Delay 0.5)
    (Rendering|Material|SetVectorParameterValue (Variables|Default|GetFlashMat) "EmissiveColor" "(R=0.000000,G=0.000000,B=0.000000,A=1.000000)" :!class /Script/Engine.MaterialInstanceDynamic)
    (Rendering|Material|SetScalarParameterValue (Variables|Default|GetFlashMat) "EmissiveMultiplier" 0.0 :!class /Script/Engine.MaterialInstanceDynamic)))

(event EventBeginPlay
  (bind _returnvalue (Components|GetOwner))
  (Variables|Default|SetOwner _returnvalue)
  (Collision|BindEventtoOnActorBeginOverlap _returnvalue (EventDispatchers|CreateEvent :!event Custom|FlashRed))
  (Utilities|IsValid (Actor|GetComponentbyClass (Variables|Default|GetOwner) "/Script/Engine.SkeletalMeshComponent")
    (:Is%20Valid
      (bind _returnvalue_2 (Rendering|Material|CreateDynamicMaterialInstance (Actor|GetComponentbyClass (Variables|Default|GetOwner) "/Script/Engine.SkeletalMeshComponent") 0 0 "None" :!class /Script/Engine.PrimitiveComponent))
      (Variables|Default|SetFlashMat _returnvalue_2))))